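; Player controller that turns axis inputs into look and movement for the possessed pawn.
; BeginPlay caches the controlled pawn and a BP_Player-typed reference, which the graph does not use afterwards.
; Turn and LookUp apply raw yaw and pitch, while their Rate variants scale by world delta time.
; Forward and right movement follow only the control rotation's yaw, keeping movement input on the horizontal plane.
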(event `self.ReceiveBeginPlay`
  (bind _returnvalue (`self.K2_GetPawn`))
  (set `self.MyPlayer` _returnvalue)
  (bind _asbp_player (cast `/Game/GameFolder/Player_Blueprints/BP_Player` _returnvalue))
  (set `self.MyPlayer_BP` _asbp_player))

(event `InputAxis|TurnRate`
  (params (AxisValue :type "Float (single-precision)"))
  (`Pawn.AddControllerYawInput` (`self.MyPlayer`) (* AxisValue (`GameplayStatics.GetWorldDeltaSeconds`))))

(event `InputAxis|LookUpRate`
  (params (AxisValue :type "Float (single-precision)"))
  (`Pawn.AddControllerPitchInput` (`self.MyPlayer`) (* AxisValue (`GameplayStatics.GetWorldDeltaSeconds`))))

(event `InputAxis|Turn` :overrideparent false
  (params (AxisValue :type "Float (single-precision)"))
  (`Pawn.AddControllerYawInput` (`self.MyPlayer`) AxisValue))

(event `InputAxis|LookUp` :overrideparent false
  (params (AxisValue :type "Float (single-precision)"))
  (`Pawn.AddControllerPitchInput` (`self.MyPlayer`) AxisValue))

(event `InputAxis|MoveForward` :overrideparent false
  (params (AxisValue :type "Float (single-precision)"))
  (`Pawn.AddMovementInput` (`self.MyPlayer`) (`KismetMathLibrary.GetForwardVector` (`KismetMathLibrary.MakeRotator` 0.0 0.0 (.yaw (`Pawn.GetControlRotation` (`self.MyPlayer`))))) AxisValue false))

(event `InputAxis|MoveRight` :overrideparent false
  (params (AxisValue :type "Float (single-precision)"))
  (`Pawn.AddMovementInput` (`self.MyPlayer`) (`KismetMathLibrary.GetRightVector` (`KismetMathLibrary.MakeRotator` 0.0 0.0 (.yaw (`Pawn.GetControlRotation` (`self.MyPlayer`))))) AxisValue false))

(fn `UserConstructionScript`)