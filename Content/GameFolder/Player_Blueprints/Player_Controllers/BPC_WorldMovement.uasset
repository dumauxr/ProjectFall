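; Player controller for world movement that also drives a fight-mode menu overlay.
; On BeginPlay it caches the controlled BP_Player pawn and creates the HUD_FightMode widget.
; The O key flip-flops the fight menu, adding or removing the widget and setting InFightMenu.
; That flag switches input between yaw-relative planar pawn movement and directional menu navigation forwarded to the widget.
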(event `self.ReceiveBeginPlay`
  (`self.setPlayer`) ; Récupère le BP du joueur et le renseigne dans deux variables, MyPlayer qui correspond à l'actor du joueur\nMyPlayer_BP référencie le Blueprint du joueur
  (bind _returnvalue (`|CreateWidget` "/Game/GameFolder/Player_Blueprints/HUD/HUD_FightMode.HUD_FightMode_C"))
  (set `self.HUD_FightMenu` _returnvalue))

(event `InputAxis|MoveForward` :overrideparent false
  (params (AxisValue :type "Float (single-precision)"))
  ;[1 1 1] Movements inputs
  (if (not (`self.inFightMenu?`))
    (`Pawn.AddMovementInput` (`self.MyPlayer`) (`KismetMathLibrary.GetForwardVector` (`KismetMathLibrary.MakeRotator` 0.0 0.0 (.yaw (`Pawn.GetControlRotation` (`self.MyPlayer`))))) AxisValue false)))

(event `InputAxis|MoveRight` :overrideparent false
  (params (AxisValue :type "Float (single-precision)"))
  ;[1 1 1] Movements inputs
  (if (not (`self.inFightMenu?`))
    (`Pawn.AddMovementInput` (`self.MyPlayer`) (`KismetMathLibrary.GetRightVector` (`KismetMathLibrary.MakeRotator` 0.0 0.0 (.yaw (`Pawn.GetControlRotation` (`self.MyPlayer`))))) AxisValue false)))

(event `InputAction|Menu_Up`
  (params (Key :type "Key Structure"))
  (:`Pressed`
    (if (`self.inFightMenu?`)
      (`/Game/GameFolder/Player_Blueprints/HUD/HUD_FightMode.navigateInMenu` (`self.HUD_FightMenu`) "NewEnumerator0"))))

(event `Key|O`
  (params (Key :type "Key Structure"))
  (:`Pressed`
    (`/Engine/EditorBlueprintResources/StandardMacros.FlipFlop`
      (:`A`
        (`self.setFightMenu` true))
      (:`B`
        (`self.setFightMenu` false)))))

(event `InputAction|Menu_Down`
  (params (Key :type "Key Structure"))
  (:`Pressed`
    (if (`self.inFightMenu?`)
      (`/Game/GameFolder/Player_Blueprints/HUD/HUD_FightMode.navigateInMenu` (`self.HUD_FightMenu`) "NewEnumerator1"))))

(event `InputAction|Menu_Left`
  (params (Key :type "Key Structure"))
  (:`Pressed`
    (if (`self.inFightMenu?`)
      (`/Game/GameFolder/Player_Blueprints/HUD/HUD_FightMode.navigateInMenu` (`self.HUD_FightMenu`) "NewEnumerator2"))))

(event `InputAction|Menu_Right`
  (params (Key :type "Key Structure"))
  (:`Pressed`
    (if (`self.inFightMenu?`)
      (`/Game/GameFolder/Player_Blueprints/HUD/HUD_FightMode.navigateInMenu` (`self.HUD_FightMenu`) "NewEnumerator3"))))

(fn `setFightMenu`
  (params (`FightMenu ?` :type Boolean))
  (bind _hud_fightmenu (`self.HUD_FightMenu`))
  (bind _output_get (set `self.inFightMenu?` `FightMenu ?`))
  (if _output_get
    (`UserWidget.AddToViewport` _hud_fightmenu 0)
    (else
      (`Widget.RemoveFromParent` _hud_fightmenu))))

(fn `setPlayer`
  (bind _returnvalue (`self.K2_GetPawn`))
  (set `self.MyPlayer` _returnvalue)
  (bind _asbp_player (cast `/Game/GameFolder/Player_Blueprints/BP_Player` _returnvalue))
  (set `self.MyPlayer_BP` _asbp_player))

(fn `UserConstructionScript`)