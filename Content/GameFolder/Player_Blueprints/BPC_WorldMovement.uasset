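; Player controller for world movement that drives the controlled pawn from movement input axes.
; On BeginPlay it caches the controlled pawn, also cast to BP_Player.
; MoveForward and MoveRight add movement input along the control rotation's yaw only, keeping movement on the horizontal plane.
; Camera turn and look-up axes are deliberately disabled, with their controller yaw and pitch logic left disconnected.
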(event `self.ReceiveBeginPlay`
  (`self.setPlayer`) ; Récupère le BP du joueur et le renseigne dans deux variables, MyPlayer qui correspond à l'actor du joueur\nMyPlayer_BP référencie le Blueprint du joueur
)

(event `InputAxis|TurnRate`
  (params (AxisValue :type "Float (single-precision)"))
  ;[1 1 1] Movement de camera - Desactivé volontairement
)

(event `InputAxis|MoveForward` :overrideparent false
  (params (AxisValue :type "Float (single-precision)"))
  ;[1 1 1] Movements inputs
  (`Pawn.AddMovementInput` (`self.MyPlayer`) (`KismetMathLibrary.GetForwardVector` (`KismetMathLibrary.MakeRotator` 0.0 0.0 (.yaw (`Pawn.GetControlRotation` (`self.MyPlayer`))))) AxisValue false))

(event `InputAxis|LookUpRate`
  (params (AxisValue :type "Float (single-precision)"))
  ;[1 1 1] Movement de camera - Desactivé volontairement
)

(event `InputAxis|Turn` :overrideparent false
  (params (AxisValue :type "Float (single-precision)"))
  ;[1 1 1] Movement de camera - Desactivé volontairement
)

(event `InputAxis|MoveRight` :overrideparent false
  (params (AxisValue :type "Float (single-precision)"))
  ;[1 1 1] Movements inputs
  (`Pawn.AddMovementInput` (`self.MyPlayer`) (`KismetMathLibrary.GetRightVector` (`KismetMathLibrary.MakeRotator` 0.0 0.0 (.yaw (`Pawn.GetControlRotation` (`self.MyPlayer`))))) AxisValue false))

(event `InputAxis|LookUp` :overrideparent false
  (params (AxisValue :type "Float (single-precision)"))
  ;[1 1 1] Movement de camera - Desactivé volontairement
)

(fn `setPlayer`
  (bind _returnvalue (`self.K2_GetPawn`))
  (set `self.MyPlayer` _returnvalue)
  (bind _asbp_player (cast `/Game/GameFolder/Player_Blueprints/BP_Player` _returnvalue))
  (set `self.MyPlayer_BP` _asbp_player))

(fn `UserConstructionScript`)