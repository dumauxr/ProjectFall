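; BP_AttackController spawns a BP_Attack between a given start and end point when AttackEvent fires.
; It places the attack at the Start component, passes a fixed speed and a direction vector aimed at the End component, and stores the new instance.
; Two helper functions compute an actor-to-component offset and scale it by a percentage, though the event does not call them.
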(event `Attack Event`
  (params (`Attack Start` :type "/Game/GameFolder/Fight_Blueprints/BP_AttackLocations Object Reference") (`Attack End` :type "/Game/GameFolder/Fight_Blueprints/BP_AttackLocations Object Reference"))
  (bind _returnvalue (`SceneComponent.K2_GetComponentLocation` (`/Game/GameFolder/Fight_Blueprints/BP_AttackLocations.Start` `Attack Start`)))
  (bind _returnvalue_2 (`|SpawnActorFromClass` "/Game/GameFolder/Fight_Blueprints/BP_Attack.BP_Attack_C" (`KismetMathLibrary.MakeTransform` _returnvalue) "Undefined" "OverrideRootScale" null 500.0 (`KismetMathLibrary.GetForwardVector` (`KismetMathLibrary.FindLookAtRotation` _returnvalue (`SceneComponent.K2_GetComponentLocation` (`/Game/GameFolder/Fight_Blueprints/BP_AttackLocations.End` `Attack End`)))) null))
  (set `self.Attack` _returnvalue_2))

(fn `getDistance`
  (params (Actor :type "Actor Object Reference") (`Scene Object` :type "SceneComponent Object Reference"))
  (returns (Result :type "Vector Structure"))
  (return (- (`SceneComponent.K2_GetComponentLocation` `Scene Object`) (`self.K2_GetActorLocation` Actor))))

(fn `getLocation`
  (params (Actor :type "Actor Object Reference") (Distance :type "Vector Structure") (Percent :type "Float (double-precision)"))
  (returns (Location :type "Vector Structure"))
  (return (* Distance Percent)))

(fn `UserConstructionScript`)